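; Player kart driven by physics forces on a box body, using Enhanced Input for throttle, steering, boost and air tricks.
; Each tick, a line trace per wheel applies spring-like suspension force, moves the wheel visual and, on contact, adds forward drive force.
; Throttle input is smoothed, decays over time and spins the wheels; steering applies throttle-scaled yaw torque.
; Boost briefly overrides throttle with a Niagara effect, and airborne tricks apply a steer-scaled impulse.
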(event `EnhancedInput|/Game/RafaAssets/Inputs/IA_Accelerate`
  (params (ActionValue :type "Float (double-precision)") (ElapsedSeconds :type "Float (double-precision)") (TriggeredSeconds :type "Float (double-precision)") (InputAction :type "InputAction Object Reference" :default "/Game/RafaAssets/Inputs/IA_Accelerate.IA_Accelerate"))
  (:`Triggered`
    (set `self.AccelerationInput` (`KismetMathLibrary.FInterpTo` (`self.AccelerationInput`) (`KismetMathLibrary.SelectFloat` ActionValue (* ActionValue 0.9) (`self.IsOnGround`)) (`GameplayStatics.GetWorldDeltaSeconds`) 0.5))))

(event `self.ReceiveBeginPlay`
  ; Inicio de kart
  (`EnhancedInputSubsystemInterface.AddMappingContext` (pcsubsystem `EnhancedInputLocalPlayerSubsystem` (`GameplayStatics.GetPlayerController` 0)) "/Game/RafaAssets/Inputs/IMC_Vehicle.IMC_Vehicle" 0 (struct)))

(event `EnhancedInput|/Game/RafaAssets/Inputs/IA_Boost`
  (params (ActionValue :type Boolean) (ElapsedSeconds :type "Float (double-precision)") (TriggeredSeconds :type "Float (double-precision)") (InputAction :type "InputAction Object Reference" :default "/Game/RafaAssets/Inputs/IA_Boost.IA_Boost"))
  (:`Started`
    (`ActorComponent.Activate` (`self.NewNiagaraSystem`) false)
    (set `self.AccelerationInput` (`self.boostAccel`))
    (`KismetSystemLibrary.Delay` 0.5)
    (set `self.AccelerationInput` (`self.normalAccel`))
    (`ActorComponent.Deactivate` (`self.NewNiagaraSystem`))))

(event `self.ReceiveTick`
  (params (DeltaSeconds :type "Float (single-precision)"))
  ; Suspensión en cada llanta
  (`self.SuspensionCast` (`self.left_wheel`))
  (`self.SuspensionCast` (`self.right_wheel`))
  (`self.SuspensionCast` (`self.Bleft_wheel`))
  (`self.SuspensionCast` (`self.Bright_wheel`))
  (`self.CalculateAcceleration`))

(event `EnhancedInput|/Game/RafaAssets/Inputs/IA_Steer`
  (params (ActionValue :type "Float (double-precision)") (ElapsedSeconds :type "Float (double-precision)") (TriggeredSeconds :type "Float (double-precision)") (InputAction :type "InputAction Object Reference" :default "/Game/RafaAssets/Inputs/IA_Steer.IA_Steer"))
  ; Steering en las dos ruedas delanteras
  (:`Triggered`
    (`PrimitiveComponent.AddTorqueInRadians` (`self.Box`) (`KismetMathLibrary.MakeVector` 0.0 0.0 (* (* ActionValue (`self.AccelerationInput`)) 10000000.0)) "None" false)))

(event `EnhancedInput|/Game/VehicleTemplate/Input/Actions/IA_AirTrick`
  (params (ActionValue :type Boolean) (ElapsedSeconds :type "Float (double-precision)") (TriggeredSeconds :type "Float (double-precision)") (InputAction :type "InputAction Object Reference" :default "/Game/VehicleTemplate/Input/Actions/IA_AirTrick.IA_AirTrick"))
  (:`Triggered`
    (`self.AirTricks`)))

(fn `AirTricks`
  (if (not (`self.IsOnGround`))
    (`PrimitiveComponent.AddVelocityChangeImpulseAtLocation` (`self.SKM_SportsCar`) (* (0.15 0.0 0.0) (`|GetInputActionValue`)) (0.0 0.0 0.0) "None")
    (`KismetSystemLibrary.PrintString` (`KismetStringLibrary.Conv_DoubleToString` (`|GetInputActionValue`)))))

(fn `CalculateAcceleration`
  (bind _accelerationinput (`self.AccelerationInput`))
  (bind _output_get (set `self.Acceleration` (* (`KismetMathLibrary.Lerp` 0.0 15000.0 _accelerationinput) _accelerationinput)))
  (set `self.AccelerationInput` (`KismetMathLibrary.FInterpTo` (`self.AccelerationInput`) 0.0 (`GameplayStatics.GetWorldDeltaSeconds`) 0.3))
  (`SceneComponent.K2_AddLocalRotation` (`self.Wheel_BLeft`) (`KismetMathLibrary.MakeRotator` 0.0 (/ _output_get -1000.0)) false false)
  (`SceneComponent.K2_AddLocalRotation` (`self.Wheel_Left`) (`KismetMathLibrary.MakeRotator` 0.0 (/ _output_get -1000.0)) false false)
  (`SceneComponent.K2_AddLocalRotation` (`self.Wheel_BRight`) (`KismetMathLibrary.MakeRotator` 0.0 (/ _output_get -1000.0)) false false)
  (`SceneComponent.K2_AddLocalRotation` (`self.Wheel_Right`) (`KismetMathLibrary.MakeRotator` 0.0 (/ _output_get -1000.0)) false false))

(fn `IsOnGround`
  (returns (ReturnValue :type Boolean))
  (bind _returnvalue (`self.K2_GetActorLocation`))
  (bind (_outhit _returnvalue_2) (`KismetSystemLibrary.LineTraceSingle` _returnvalue (- _returnvalue (0.0 0.0 20.0)) "TraceTypeQuery1"))
  (return _returnvalue_2))

(fn `KartAcceleration`
  (params (`Wheel Comp` :type "SceneComponent Object Reference"))
  (bind _box (`self.Box`))
  (`PrimitiveComponent.AddForceAtLocation` (`self.Box`) (* (`SceneComponent.GetForwardVector` _box) 5000.0 (`self.AccelerationInput`) (`PrimitiveComponent.GetMass` _box)) (`SceneComponent.K2_GetComponentLocation` `Wheel Comp`) "None"))

(fn `SuspensionCast`
  (params (WheelComp :type "SceneComponent Object Reference"))
  (bind _returnvalue (`SceneComponent.K2_GetComponentLocation` WheelComp))
  (bind _returnvalue_2 (`SceneComponent.GetChildComponent` (`local.WheelComp`) 0))
  (bind (_relativelocation_x _relativelocation_y _relativelocation_z) (`KismetMathLibrary.BreakVector` (`SceneComponent.RelativeLocation` _returnvalue_2)))
  (bind _outhit (`KismetSystemLibrary.LineTraceSingle` :`Start` _returnvalue :`End` (+ _returnvalue (* (`SceneComponent.GetUpVector` WheelComp) -60.0)) :`TraceChannel` "TraceTypeQuery2" :`bTraceComplex` true :`DrawDebugType` "Persistent"))
  (bind (_bblockinghit _binitialoverlap _time _distance _location _impactpoint _normal _impactnormal _physmat _hitactor _hitcomponent _hitbonename _bonename _hititem _elementindex _faceindex _tracestart _traceend) (`GameplayStatics.BreakHitResult` _outhit))
  ; imprime el texto y nos dice que no hace la suspensión
  (if _bblockinghit
    ; Vuelta de rueda cuando acelera o retrocede
    (`PrimitiveComponent.AddForceAtLocation` (`self.Box`) (* (- 1.0 (`KismetMathLibrary.NormalizeToRange` _distance 1.0 60.0)) (`KismetMathLibrary.GetDirectionUnitVector` _traceend _tracestart) 85000.0) (`SceneComponent.K2_GetComponentLocation` (`local.WheelComp`)) "None")
    (`self.KartAcceleration` (`local.WheelComp`))
    (`SceneComponent.K2_SetRelativeLocation` _returnvalue_2 (`KismetMathLibrary.MakeVector` 0.0 0.0 (`KismetMathLibrary.FInterpTo` _relativelocation_z (+ (* _distance -1.0) 25.0) (`GameplayStatics.GetWorldDeltaSeconds`) 3.0)) false false)))

(fn `UserConstructionScript`)