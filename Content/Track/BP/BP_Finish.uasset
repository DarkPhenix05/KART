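; Finish line actor for a kart race that counts laps and hands out finishing positions.
; On BeginPlay it sets every BP_kart's LapNumber from its Laps value.
; A box overlap adds a lap only if the kart last touched LastCheckPoint, then clears that reference and calls CheckIfFinish.
; GetPosition increments a shared index and assigns it as the given kart's finish position.
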(event `self.ReceiveBeginPlay`
  (bind _outactors (`GameplayStatics.GetAllActorsOfClass` "/Game/RafaAssets/BP_kart.BP_kart_C"))
  (for _array_element _outactors
    (set `/Game/RafaAssets/BP_kart.lapNumber` (`self.Laps`) _array_element)))

(event `self.Box.OnComponentBeginOverlap`
  (params (OverlappedComponent :type "PrimitiveComponent Object Reference") (OtherActor :type "Actor Object Reference") (OtherComp :type "PrimitiveComponent Object Reference") (OtherBodyIndex :type Integer) (bFromSweep :type Boolean) (SweepResult :type "HitResult Structure (by ref)"))
  (bind _asbp_kart (cast `/Game/RafaAssets/BP_kart` OtherActor))
  (if (== (`/Game/RafaAssets/BP_kart.lastColiderRef` _asbp_kart) (`self.LastCheckPoint`))
    (`KismetSystemLibrary.LogString` "LapCount")
    (bind _asbp_kart_2 (cast `/Game/RafaAssets/BP_kart` OtherActor))
    (`/Game/RafaAssets/BP_kart.AddLap` _asbp_kart_2 1)
    (set `/Game/RafaAssets/BP_kart.lastColiderRef` null _asbp_kart_2)
    (`/Game/RafaAssets/BP_kart.CheckIfFinish` _asbp_kart_2)
    (else
      (`KismetSystemLibrary.LogString` "Didn't touch last checkpoint"))))

(event `self.Box.OnComponentEndOverlap`
  (params (OverlappedComponent :type "PrimitiveComponent Object Reference") (OtherActor :type "Actor Object Reference") (OtherComp :type "PrimitiveComponent Object Reference") (OtherBodyIndex :type Integer))
  (`KismetSystemLibrary.Delay` 0.2)
  (`ActorComponent.Activate` (`self.Box`) false)
  (`KismetSystemLibrary.LogString` "Start Off"))

(event `GetPosition`
  (params (BPKart :type "Actor Object Reference"))
  ;[0.7344 0.6013 0 0.5] Get/Set kart Pos
  (bind _output_get (set `self.PositioningIndex` (+ (`self.PositioningIndex`) 1)))
  (bind _asbp_kart (cast `/Game/RafaAssets/BP_kart` BPKart))
  (`/Game/RafaAssets/BP_kart.SetFinishPosition` _asbp_kart _output_get))

(fn `UserConstructionScript`)