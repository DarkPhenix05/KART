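; BP_Weapon is an unfinished weapon actor with firing and contact-damage logic.
; FireWeapon spawns a BP_Weapon at its own transform as owner, then calls itself and loops back to the spawn with no exit condition.
; Collision overlap calls ApplyDamage with a fixed amount and no target connected.
; The ammo check, BP_Camaro owner cast and SpawnedWeapon reset are disconnected and never run.
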(event `FireWeapon`
  ; Weapon
  (bind _returnvalue (`|SpawnActorFromClass` "BP_Weapon_C" (`KismetMathLibrary.MakeTransform` (.location (`self.GetTransform`)) (.rotation (`self.GetTransform`)) (.scale (`self.GetTransform`))) "Undefined" "MultiplyWithRoot" self null :!label _label))
  (`self.FireWeapon`)
  (goto _label))

(event `self.CollisionComponent.OnComponentBeginOverlap`
  (params (OverlappedComponent :type "PrimitiveComponent Object Reference") (OtherActor :type "Actor Object Reference") (OtherComp :type "PrimitiveComponent Object Reference") (OtherBodyIndex :type Integer) (bFromSweep :type Boolean) (SweepResult :type "HitResult Structure (by ref)"))
  ; Damage
  (`GameplayStatics.ApplyDamage` null 25.0))

(fn `UserConstructionScript`)